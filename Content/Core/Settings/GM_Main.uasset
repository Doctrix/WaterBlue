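; Main game mode that runs the match: menu or game start, HUD, score and win/lose end screen.
; BeginPlay caches the controller, items and container, creates the HUD, briefly shows a tutorial and starts a looping timer.
; Helper functions push player stats, collected water and minerals, container status and elevator position to the HUD.
; CheckStatusGame triggers Winner on a full container slot, while reaching exactly 1000 points raises the player's level.
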(event Custom|LauchGame
  (if (Variables|Bool|GetStartGame)
    (Utilities|FlowControl|Sequence
      (:then_0
        (bind _controller (CallFunction|CastController))
        (Variables|Reference|SetController _controller)
        (bind _outactors (Actor|GetAllActorsOfClass "/Game/Core/Item/BP_Item.BP_Item_C"))
        (Variables|Default|SetItems _outactors)
        (bind _outactors_2 (Actor|GetAllActorsOfClass "/Game/Core/Container/BP_ContainerMaster.BP_ContainerMaster_C"))
        (for _array_element _outactors_2
          (Variables|Default|SetContainer _array_element)))
      (:then_1
        (bind _returnvalue (UserInterface|CreateWidget "/Game/Core/Settings/WBP_IngameHUD.WBP_IngameHUD_C"))
        (bind _output_get (Variables|Reference|SetUI_Player _returnvalue))
        (UserInterface|Viewport|AddtoViewport _output_get 0)
        (Utilities|FlowControl|Delay 5.0)
        (Widget|SetVisibility (Variables|/Game/Core/Settings/WBP_IngameHUD.WBP_IngameHUD_C|GetTextTuto _output_get) "Visible")
        (Utilities|FlowControl|Delay 1e+01)
        (Widget|SetVisibility (Variables|/Game/Core/Settings/WBP_IngameHUD.WBP_IngameHUD_C|GetTextTuto _output_get) "Collapsed"))
      (:then_2
        (CallFunction|SetupStatsPlayer)
        (CallFunction|AddNewLevel))
      (:then_3
        (Utilities|Time|SetTimerbyEvent (EventDispatchers|CreateEvent :!event UpdateGaujePositionElevator) 0.1 true)))
    (else
      (bind _returnvalue_2 (UserInterface|CreateWidget "/Game/Core/Menu/WBP_MenuMain.WBP_MenuMain_C"))
      (UserInterface|Viewport|AddtoViewport _returnvalue_2 0))))

(event Custom|GameOver
  (Variables|Bool|SetWinLose false)
  (Widget|RemovefromParent (Variables|Reference|GetUI_Player))
  (bind _returnvalue (UserInterface|CreateWidget "/Game/Core/Menu/WBP_ScreenEndGame.WBP_ScreenEndGame_C"))
  (UserInterface|Viewport|AddtoViewport _returnvalue 0))

(event Custom|Winner
  (Variables|Bool|SetWinLose true)
  (Widget|RemovefromParent (Variables|Reference|GetUI_Player))
  (bind _returnvalue (UserInterface|CreateWidget "/Game/Core/Menu/WBP_ScreenEndGame.WBP_ScreenEndGame_C"))
  (UserInterface|Viewport|AddtoViewport _returnvalue 0))

(event Custom|CheckStatusGame
  (bind _returnvalue (Game|GetPlayerController 0))
  (for _array_element (Variables|/Game/Core/Inventory/AC_InventoryMaster.AC_InventoryMaster_C|GetInventory (Variables|/Game/Core/Container/BP_ContainerMaster.BP_ContainerMaster_C|GetInventoryContainer (Variables|Default|GetContainer)))
    (if (Utilities|Struct|BreakS_Inventory _array_element)
      (Utilities|FlowControl|Delay 3.0)
      (Input|DisableInput _returnvalue _returnvalue)
      (CallFunction|Winner))))

(event Custom|ShowMsgTuto
  (Widget|SetVisibility (Variables|/Game/Core/Settings/WBP_IngameHUD.WBP_IngameHUD_C|GetTextTuto (stale Custom|LauchGame _output_get)) "Visible")
  (Utilities|FlowControl|Delay 1e+01)
  (Widget|SetVisibility (Variables|/Game/Core/Settings/WBP_IngameHUD.WBP_IngameHUD_C|GetTextTuto (stale Custom|LauchGame _output_get)) "Collapsed"))

(event EventBeginPlay
  (if (Variables|Bool|GetStartGame)
    (Utilities|FlowControl|Sequence
      (:then_0
        (bind _controller (CallFunction|CastController))
        (Variables|Reference|SetController _controller)
        (bind _outactors (Actor|GetAllActorsOfClass "/Game/Core/Item/BP_Item.BP_Item_C"))
        (Variables|Default|SetItems _outactors)
        (bind _outactors_2 (Actor|GetAllActorsOfClass "/Game/Core/Container/BP_ContainerMaster.BP_ContainerMaster_C"))
        (for _array_element _outactors_2
          (Variables|Default|SetContainer _array_element)))
      (:then_1
        (bind _returnvalue (UserInterface|CreateWidget "/Game/Core/Settings/WBP_IngameHUD.WBP_IngameHUD_C"))
        (bind _output_get (Variables|Reference|SetUI_Player _returnvalue))
        (UserInterface|Viewport|AddtoViewport _output_get 0)
        (Utilities|FlowControl|Delay 5.0)
        (Widget|SetVisibility (Variables|/Game/Core/Settings/WBP_IngameHUD.WBP_IngameHUD_C|GetTextTuto _output_get) "Visible")
        (Utilities|FlowControl|Delay 1e+01)
        (Widget|SetVisibility (Variables|/Game/Core/Settings/WBP_IngameHUD.WBP_IngameHUD_C|GetTextTuto _output_get) "Collapsed"))
      (:then_2
        (CallFunction|SetupStatsPlayer)
        (CallFunction|AddNewLevel))
      (:then_3
        (Utilities|Time|SetTimerbyEvent (EventDispatchers|CreateEvent :!event UpdateGaujePositionElevator) 0.1 true)))
    (else
      (bind _returnvalue_2 (UserInterface|CreateWidget "/Game/Core/Menu/WBP_MenuMain.WBP_MenuMain_C"))
      (UserInterface|Viewport|AddtoViewport _returnvalue_2 0))))

(fn ConstructionScript)

(fn UpdateGaujePositionElevator
  (bind _returnvalue (Actor|GetActorOfClass "/Game/Core/Elevator/BP_Elevator.BP_Elevator_C"))
  (Default|SetGaujeElevator (Variables|Reference|GetUI_Player) (Variables|/Game/Core/Elevator/BP_Elevator.BP_Elevator_C|GetPosZ _returnvalue))
  (return))

(fn AddOnePoints
  (bind _result (Math|Integer|IncrementInt (Variables|Default|GetPoints))
    (:%20%20
      (Default|SetPlayerScore (Variables|Reference|GetUI_Player) _result)
      (CallFunction|AddNewLevel)
      (return))))

(fn IncrementMineralCollectPlayer
  (params (Mine :type Float%20%28single-precision%29))
  (Default|SetPlayerCollectMineral (Variables|Reference|GetUI_Player) Mine)
  (return))

(fn DecrementMineralCollectPlayer
  (Default|SetPlayerCollectMineral (Variables|Reference|GetUI_Player) 0.0)
  (return))

(fn IncrementWaterCollectPlayer
  (params (Value :type Float%20%28single-precision%29))
  (Default|SetPlayerCollectWater (Variables|Reference|GetUI_Player) Value)
  (return))

(fn DecrementWaterCollectPlayer
  (Default|SetPlayerCollectWater (Variables|Reference|GetUI_Player) 0.0)
  (return))

(fn IncrementMineralContainer
  (params (Name :type String) (amonut :type Float%20%28single-precision%29) (max :type Float%20%28single-precision%29))
  (Default|SetStatusMineral (Variables|Reference|GetUI_Player) Name amonut max)
  (return))

(fn IncrementWaterContainer
  (params (Name :type String) (amonut :type Float%20%28single-precision%29) (max :type Float%20%28single-precision%29))
  (Default|SetStatusWater (Variables|Reference|GetUI_Player) Name amonut max)
  (return))

(fn SetupStatsPlayer
  (bind _ui_player (Variables|Reference|GetUI_Player))
  (bind _controller (Variables|Reference|GetController))
  (bind _playerstats (Variables|/Game/Core/Player/PC_Ingame.PC_Ingame_C|GetPlayerStats _controller))
  (bind _inventoryplayer (Variables|/Game/Core/Player/PC_Ingame.PC_Ingame_C|GetInventoryPlayer _controller))
  (bind (_name _health _level) (Utilities|Struct|BreakS_PlayerStats _playerstats))
  (bind _inventory (Variables|/Game/Core/Inventory/AC_InventoryMaster.AC_InventoryMaster_C|GetInventory _inventoryplayer))
  (bind _output (Utilities|Array|Get(acopy) _inventory))
  (bind _quantity (Utilities|Struct|BreakS_Inventory _output))
  (Default|SetPlayerCollectWater _ui_player _quantity)
  (Default|SetPlayerCollectMineral _ui_player _quantity)
  (Default|SetPlayerName _ui_player (Utilities|Text|ToText(Name) _name))
  (Default|SetPlayerHealth _ui_player _health)
  (Default|SetPlayerLevel _ui_player _level))

(fn AddNewLevel
  (bind _controller (Variables|Reference|GetController))
  (bind _playerstats (Variables|/Game/Core/Player/PC_Ingame.PC_Ingame_C|GetPlayerStats _controller))
  (if (== (Variables|Default|GetPoints) 1000)
    (bind _structout (Utilities|Struct|SetmembersinS_PlayerStats _playerstats (+ (Variables|Default|GetAddLevel) (Utilities|Struct|BreakS_PlayerStats _playerstats))))
    (Default|SetPlayerLevel (Variables|Reference|GetUI_Player) (Utilities|Struct|BreakS_PlayerStats _structout))
    (return)))

(fn GetGameMode
  (return self))