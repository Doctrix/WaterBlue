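; In-game player controller that opens the pause menu when P is pressed.
; The P handler creates and stores a new WBP_MenuPause, adds it to the viewport, switches input mode and pauses the game.
; ModeGameAndOnly sets Game and UI input with a visible cursor, while ModeGameOnly restores game-only input and hides it.
; GetController returns the controller itself; unpausing is not handled here.
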(event EventBeginPlay)

(event EventTick
  (params (DeltaSeconds :type Float%20%28single-precision%29)))

(event Input|KeyboardEvents|P
  (params (Key :type Key%20Structure))
  (:Pressed
    (bind _returnvalue (UserInterface|CreateWidget "/Game/Core/Menu/WBP_MenuPause.WBP_MenuPause_C"))
    (bind _output_get (Variables|Default|SetPauseMenuScreen _returnvalue))
    (UserInterface|Viewport|AddtoViewport _output_get 0)
    (CallFunction|ModeGameandOnly (Variables|Default|GetPauseMenuScreen))
    (Game|SetGamePaused true)))

(fn ConstructionScript)

(fn ModeGameandOnly
  (params (InWidgetToFocus :type Widget%20Object%20Reference))
  (Input|SetInputModeGameandUI self InWidgetToFocus "DoNotLock" false)
  (Variables|Default|SetbShowMouseCursor true)
  (return))

(fn ModeGameOnly
  (Input|SetInputModeGameOnly self)
  (Variables|Default|SetbShowMouseCursor false)
  (return))

(fn GetController
  (return self))