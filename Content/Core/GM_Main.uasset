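; Main game mode that shows either the main menu or the in-game HUD, depending on StartGame.
; It caches the player controller, seeds the HUD from its stats and inventory, and starts a looping timer.
; Helper functions update score, collected water and minerals, mineral container status and the elevator gauge, pushing values to the HUD.
; LauchGame re-runs the startup branch; IncrementWaterContainer is an empty stub.
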(event Custom|LauchGame
  (if (Variables|Default|GetStartGame)
    (bind _controller (CallFunction|CastController))
    (Variables|Reference|SetController _controller)
    (bind _returnvalue (UserInterface|CreateWidget "/Game/Core/HUD/WBP_IngameHUD.WBP_IngameHUD_C"))
    (bind _output_get (Variables|Reference|SetUI_Player _returnvalue))
    (UserInterface|Viewport|AddtoViewport _output_get 0)
    (Utilities|FlowControl|Sequence
      (:then_0
        (Utilities|Time|SetTimerbyEvent (EventDispatchers|CreateEvent :!event UpdateGaujePositionElevator) 0.1 true))
      (:then_1
        (Default|SetPlayerCollectWater (Variables|Reference|GetUI_Player) (Variables|/Game/Core/Player/AC_Inventory.AC_Inventory_C|GetQuantityWaterCollected (Variables|/Game/Core/Player/PC_Ingame.PC_Ingame_C|GetAC_Inventory (Variables|Reference|GetController))))
        (Default|SetPlayerCollectMineral (Variables|Reference|GetUI_Player) (Variables|/Game/Core/Player/AC_Inventory.AC_Inventory_C|GetQuantityMineralsCollected (Variables|/Game/Core/Player/PC_Ingame.PC_Ingame_C|GetAC_Inventory (Variables|Reference|GetController))))
        (Default|SetPlayerName (Variables|Reference|GetUI_Player) (Utilities|Text|ToText(Name) (.Name (Utilities|Struct|BreakS_PlayerStats (Variables|/Game/Core/Player/PC_Ingame.PC_Ingame_C|GetPlayerStats (Variables|Reference|GetController))))))
        (Default|SetPlayerHealth (Variables|Reference|GetUI_Player) (.Health (Utilities|Struct|BreakS_PlayerStats (Variables|/Game/Core/Player/PC_Ingame.PC_Ingame_C|GetPlayerStats (Variables|Reference|GetController)))))))
    (else
      (bind _returnvalue_2 (UserInterface|CreateWidget "/Game/Core/HUD/WBP_MenuMain.WBP_MenuMain_C"))
      (UserInterface|Viewport|AddtoViewport _returnvalue_2 0))))

(event EventBeginPlay
  (if (Variables|Default|GetStartGame)
    (bind _controller (CallFunction|CastController))
    (Variables|Reference|SetController _controller)
    (bind _returnvalue (UserInterface|CreateWidget "/Game/Core/HUD/WBP_IngameHUD.WBP_IngameHUD_C"))
    (bind _output_get (Variables|Reference|SetUI_Player _returnvalue))
    (UserInterface|Viewport|AddtoViewport _output_get 0)
    (Utilities|FlowControl|Sequence
      (:then_0
        (Utilities|Time|SetTimerbyEvent (EventDispatchers|CreateEvent :!event UpdateGaujePositionElevator) 0.1 true))
      (:then_1
        (Default|SetPlayerCollectWater (Variables|Reference|GetUI_Player) (Variables|/Game/Core/Player/AC_Inventory.AC_Inventory_C|GetQuantityWaterCollected (Variables|/Game/Core/Player/PC_Ingame.PC_Ingame_C|GetAC_Inventory (Variables|Reference|GetController))))
        (Default|SetPlayerCollectMineral (Variables|Reference|GetUI_Player) (Variables|/Game/Core/Player/AC_Inventory.AC_Inventory_C|GetQuantityMineralsCollected (Variables|/Game/Core/Player/PC_Ingame.PC_Ingame_C|GetAC_Inventory (Variables|Reference|GetController))))
        (Default|SetPlayerName (Variables|Reference|GetUI_Player) (Utilities|Text|ToText(Name) (.Name (Utilities|Struct|BreakS_PlayerStats (Variables|/Game/Core/Player/PC_Ingame.PC_Ingame_C|GetPlayerStats (Variables|Reference|GetController))))))
        (Default|SetPlayerHealth (Variables|Reference|GetUI_Player) (.Health (Utilities|Struct|BreakS_PlayerStats (Variables|/Game/Core/Player/PC_Ingame.PC_Ingame_C|GetPlayerStats (Variables|Reference|GetController)))))))
    (else
      (bind _returnvalue_2 (UserInterface|CreateWidget "/Game/Core/HUD/WBP_MenuMain.WBP_MenuMain_C"))
      (UserInterface|Viewport|AddtoViewport _returnvalue_2 0))))

(fn ConstructionScript)

(fn UpdateGaujePositionElevator
  (bind _returnvalue (Actor|GetActorOfClass "/Game/Core/Elevator/BP_Elevator.BP_Elevator_C"))
  (Default|SetGaujeElevator (Variables|Reference|GetUI_Player) (Variables|/Game/Core/Elevator/BP_Elevator.BP_Elevator_C|GetPosZ _returnvalue))
  (return))

(fn AddOnePoints
  (bind _result (Math|Integer|IncrementInt (Variables|Default|GetPoints))
    (:%20%20
      (Default|SetPlayerScore (Variables|Reference|GetUI_Player) _result)
      (return))))

(fn IncrementMineralCollectPlayer
  (bind _result (Math|Float|IncrementFloat (Variables|/Game/Core/Player/AC_Inventory.AC_Inventory_C|GetQuantityMineralsCollected (Variables|/Game/Core/Player/PC_Ingame.PC_Ingame_C|GetAC_Inventory (Variables|Reference|GetController))))
    (:%20%20
      (Default|SetPlayerCollectMineral (Variables|Reference|GetUI_Player) _result)
      (return))))

(fn DecrementMineralCollectPlayer
  (bind _output_get (Variables|/Game/Core/Player/AC_Inventory.AC_Inventory_C|SetQuantityMineralsCollected (Variables|/Game/Core/Player/PC_Ingame.PC_Ingame_C|GetAC_Inventory (Variables|Reference|GetController)) 0.0))
  (Default|SetPlayerCollectMineral (Variables|Reference|GetUI_Player) _output_get)
  (return))

(fn IncrementWaterCollectPlayer
  (bind _result (Math|Float|IncrementFloat (Variables|/Game/Core/Player/AC_Inventory.AC_Inventory_C|GetQuantityWaterCollected (Variables|/Game/Core/Player/PC_Ingame.PC_Ingame_C|GetAC_Inventory (Variables|Reference|GetController))))
    (:%20%20
      (Default|SetPlayerCollectWater (Variables|Reference|GetUI_Player) _result)
      (return))))

(fn DecrementWaterCollectPlayer
  (params (Quantity :type Float%20%28single-precision%29))
  (bind _controller (Variables|Reference|GetController))
  (bind _ac_inventory (Variables|/Game/Core/Player/PC_Ingame.PC_Ingame_C|GetAC_Inventory _controller))
  (bind _quantitywatercollected (Variables|/Game/Core/Player/AC_Inventory.AC_Inventory_C|GetQuantityWaterCollected _ac_inventory))
  (bind _result (Math|Float|DecrementFloat _quantitywatercollected)
    (:%20%20
      (Default|SetPlayerCollectWater (Variables|Reference|GetUI_Player) _result)
      (Water|IncrementWaterContainer (+ _quantitywatercollected Quantity))
      (return))))

(fn IncrementMineralContainer
  (params (QuantityContainer :type Float%20%28single-precision%29))
  (bind _controller (Variables|Reference|GetController))
  (bind _ac_inventory (Variables|/Game/Core/Player/PC_Ingame.PC_Ingame_C|GetAC_Inventory _controller))
  (bind _quantitymineralscollected (Variables|/Game/Core/Player/AC_Inventory.AC_Inventory_C|GetQuantityMineralsCollected _ac_inventory))
  (bind _returnvalue (+ _quantitymineralscollected QuantityContainer))
  (Default|SetQuantity (Variables|/Game/Core/HUD/WBP_IngameHUD.WBP_IngameHUD_C|GetStatusContainerMinerals (Variables|Reference|GetUI_Player)) "NewEnumerator0" _returnvalue 0.0)
  (return _returnvalue))

(fn IncrementWaterContainer
  (params (Quantity :type Float%20%28single-precision%29))
  (return))

(fn GetGameMode
  (return self))