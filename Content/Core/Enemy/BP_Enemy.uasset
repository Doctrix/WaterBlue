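; BP_Enemy is a short-lived enemy actor that damages the player on overlap and destroys itself five seconds after spawning.
; On BeginPlay it caches GM_Main plus the player controller and character, then starts the lifetime delay.
; Overlapping that character subtracts one Health from the controller's PlayerStats struct.
; If the game mode's UIPlayer is valid, it updates the health display and destroys the enemy immediately.
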(event EventBeginPlay
  (Utilities|FlowControl|Sequence
    (:then_0
      (bind _asgm_main (Utilities|Casting|CastToGM_Main (Game|GetGameMode)))
      (Variables|Reference|SetGameMode _asgm_main)
      (bind _controller (CallFunction|CastController))
      (Variables|Reference|SetController _controller)
      (bind _character (CallFunction|CastCharacter))
      (Variables|Reference|SetCharacter _character))
    (:then_1
      (Utilities|FlowControl|Delay 5.0)
      (Actor|DestroyActor))))

(event Collision|EventActorBeginOverlap
  (params (OtherActor :type Actor%20Object%20Reference))
  (bind _controller (Variables|Reference|GetController))
  (bind _playerstats (Variables|/Game/Core/Player/PC_Ingame.PC_Ingame_C|GetPlayerStats _controller))
  (if (== OtherActor (Variables|Reference|GetCharacter))
    (bind _structout (Utilities|Struct|SetmembersinS_PlayerStats _playerstats (- (Utilities|Struct|BreakS_PlayerStats _playerstats) 1.0)))
    (bind _ui_player (Variables|/Game/Core/Settings/GM_Main.GM_Main_C|GetUI_Player (Variables|Reference|GetGameMode))
      (:then
        (Default|SetPlayerHealth _ui_player (Utilities|Struct|BreakS_PlayerStats _structout))
        (Actor|DestroyActor))
      (:else))))

(fn ConstructionScript)