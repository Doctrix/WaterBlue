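; BP_Enemy is a projectile-driven enemy that costs the player one health on overlap.
; BeginPlay caches game mode, controller and character, traces toward the player, and on a blocking hit randomizes projectile InitialSpeed after a short delay.
; Overlapping the player updates PlayerStats and, with a valid UI, refreshes health, plays an explosion sound and jumps into the destroy sequence.
; That sequence, also timed from spawn, destroys the actor, adds Niagara and clears SpawnEnemy.
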(event Custom|DestroyActorFX
  (Utilities|FlowControl|Delay 2.0)
  (Actor|DestroyActor)
  (AddComponent|AddNiagaraComponent false)
  (Variables|Default|SetSpawnEnemy false))

(event EventBeginPlay
  (Utilities|FlowControl|Sequence
    (:then_0
      (bind _gamemode (CallFunction|CastGameMode))
      (Variables|Reference|SetGameMode _gamemode)
      (bind _controller (CallFunction|CastController))
      (Variables|Reference|SetController _controller)
      (bind _character (CallFunction|CastCharacter))
      (Variables|Reference|SetCharacter _character))
    (:then_1
      (bind _outhit (Collision|LineTraceByChannel (Transformation|GetActorLocation) (Transformation|GetActorLocation (Game|GetPlayerCharacter 0)) "TraceTypeQuery1" false 0 "None"))
      (Utilities|FlowControl|Delay 0.5)
      (if (.bBlockingHit (Collision|BreakHitResult _outhit))
        (Variables|/Script/Engine.ProjectileMovementComponent|SetInitialSpeed (Variables|Default|GetProjectileMovement) (Math|Random|RandomFloatinRange 1e+03 1.6e+03))))
    (:then_2
      (CallFunction|DestroyActorFX))))

(event Collision|EventActorBeginOverlap
  (params (OtherActor :type Actor%20Object%20Reference))
  (bind _controller (Variables|Reference|GetController))
  (bind _playerstats (Variables|/Game/Core/Player/PC_Ingame.PC_Ingame_C|GetPlayerStats _controller))
  (if (== OtherActor (Variables|Reference|GetCharacter))
    (bind _structout (Utilities|Struct|SetmembersinS_PlayerStats _playerstats (- (Utilities|Struct|BreakS_PlayerStats _playerstats) 1.0)))
    (bind _ui_player (Variables|/Game/Core/Settings/GM_Main.GM_Main_C|GetUI_Player (Variables|Reference|GetGameMode))
      (:then
        (Default|SetPlayerHealth _ui_player (Utilities|Struct|BreakS_PlayerStats _structout))
        (Audio|SpawnSoundatLocation "/Game/Core/Actor/Enemy/ExplosionFeu_Cue.ExplosionFeu_Cue" (Transformation|GetWorldLocation (Variables|Default|GetSphere)) "0, 0, 0" 1.0 1.0 0.0 0 0)
        (Actor|DestroyActor)
        (AddComponent|AddNiagaraComponent false)
        (Variables|Default|SetSpawnEnemy false))
      (:else))))

(fn ConstructionScript)