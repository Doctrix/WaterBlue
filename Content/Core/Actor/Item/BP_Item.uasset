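; Collectible pickup actor whose Type, Mineral or Water, selects the scaled mesh and material built in the construction script.
; When the player character overlaps it and that resource is below its max, it adds Amount to the Controller's count, notifies the GameMode, plays a sound and awards points.
; EffectDestroyActor then destroys it and adds a per-type Niagara component, as also happens automatically after a fixed delay from BeginPlay.
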(event EventBeginPlay
  (Utilities|FlowControl|Sequence
    (:then_0
      (bind _gamemode (CallFunction|CastGameMode))
      (Variables|Reference|SetGameMode _gamemode)
      (bind _character (CallFunction|CastCharacter))
      (Variables|Reference|SetCharacter _character)
      (bind _controller (CallFunction|CastController))
      (Variables|Reference|SetController _controller))
    (:then_1
      (Utilities|FlowControl|Delay 2e+01)
      (CallFunction|EffectDestroyActor))))

(event Collision|EventActorBeginOverlap
  (params (OtherActor :type Actor%20Object%20Reference))
  (bind _controller (Variables|Reference|GetController))
  (bind _gamemode (Variables|Reference|GetGameMode))
  (if (== OtherActor (Variables|Reference|GetCharacter))
    (switch Utilities|FlowControl|Switch|SwitchonE_Type (Variables|Default|GetType)
      (:NewEnumerator0
        (if (< (Variables|/Game/Core/Player/PC_Ingame.PC_Ingame_C|GetMine _controller) (Variables|/Game/Core/Player/PC_Ingame.PC_Ingame_C|GetMineMax _controller))
          (bind _output_get (Variables|/Game/Core/Player/PC_Ingame.PC_Ingame_C|SetMine _controller (+ (Variables|/Game/Core/Player/PC_Ingame.PC_Ingame_C|GetMine _controller) (Variables|Default|GetAmount))))
          (Default|IncrementMineralCollectPlayer _gamemode _output_get)
          (Audio|SpawnSoundAttached "/Game/Core/Actor/Mineral/EclatMine.EclatMine" (Variables|Default|GetDefaultSceneRoot) "None" "0, 0, 0" "0, 0, 0" "KeepWorldPosition" false 0.09 1.0 0.0 0 0)
          (Default|AddOnePoints _gamemode :!label _label)
          (CallFunction|EffectDestroyActor)))
      (:NewEnumerator2
        (if (< (Variables|/Game/Core/Player/PC_Ingame.PC_Ingame_C|GetWater _controller) (Variables|/Game/Core/Player/PC_Ingame.PC_Ingame_C|GetWaterMax _controller))
          (bind _output_get_2 (Variables|/Game/Core/Player/PC_Ingame.PC_Ingame_C|SetWater _controller (+ (Variables|/Game/Core/Player/PC_Ingame.PC_Ingame_C|GetWater _controller) (Variables|Default|GetAmount))))
          (Default|IncrementWaterCollectPlayer _gamemode _output_get_2)
          (Audio|SpawnSoundAttached "/Game/Core/Actor/Water/goutteEau.goutteEau" (Variables|Default|GetSphereWater) "None" "0, 0, 0" "0, 0, 0" "KeepWorldPosition" false 0.09 1.0 0.0 0 0)
          (goto _label))))))

(fn ConstructionScript
  (switch Utilities|FlowControl|Switch|SwitchonE_Type (Variables|Default|GetType)
    (:NewEnumerator0
      (bind _returnvalue (AddComponent|AddStaticMeshComponent false))
      (Transformation|SetRelativeScale3D _returnvalue "0.200000,0.200000,0.200000")
      (Rendering|Material|SetMaterial _returnvalue 0 "/Game/Core/Actor/Mineral/MI_Mineral.MI_Mineral"))
    (:NewEnumerator2
      (bind _returnvalue_2 (AddComponent|AddStaticMeshComponent false))
      (Variables|Default|SetSphereWater _returnvalue_2)
      (Transformation|SetRelativeScale3D _returnvalue_2 "0.200000,0.200000,0.200000")
      (Rendering|Material|SetMaterial _returnvalue_2 0 "/Game/Core/Actor/Water/MI_Water.MI_Water"))))

(fn EffectDestroyActor
  (Actor|DestroyActor)
  (switch Utilities|FlowControl|Switch|SwitchonE_Type (Variables|Default|GetType)
    (:NewEnumerator0
      (AddComponent|AddNiagaraComponent false))
    (:NewEnumerator2
      (bind _returnvalue (AddComponent|AddNiagaraComponent false))
      (Transformation|AttachComponentToComponent _returnvalue (Variables|Default|GetSphereWater) "None" "SnapToTarget" "SnapToTarget" "SnapToTarget" true)))
  (return))