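; Base resource container actor where the player deposits collected minerals or water, selected by its Type.
; The construction script adds a trigger box and platform mesh, which sinks while the player overlaps it.
; Stepping on transfers the controller's carried resource into the container, updating its status widget and GameMode totals.
; Each overlap also sets DownActive on the BP_Elevator and blinks the matching left or right character widget.
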(event Custom|IncrementResourceContainer
  (bind _playercontroller (Variables|Reference|GetPlayerController))
  (bind _gamemode (Variables|Reference|GetGameMode))
  (bind _statuscontainerwidget (Variables|Reference|GetStatusContainerWidget))
  (switch Utilities|FlowControl|Switch|SwitchonE_Type (Variables|Stats|GetType)
    (:NewEnumerator0
      (if (>= (Variables|Mine|GetQuantityMine) (Variables|Stats|GetQuantityMax))
        (Variables|Mine|SetQuantityMine (Variables|Stats|GetQuantityMax))
        (bind _output_get (Variables|Mine|SetbIsFullMine true))
        (Development|PrintString (Utilities|String|ToString(Boolean) _output_get))
        (Default|SetColorWidget (Variables|Reference|GetStatusContainerWidget) (Variables|Stats|GetType) :!label _label)
        (elif (<= (Variables|/Game/Core/Player/PC_Ingame.PC_Ingame_C|GetMine _playercontroller) 0.0)
          (goto _label)
          (elif (< (Variables|/Game/Core/Player/PC_Ingame.PC_Ingame_C|GetMine _playercontroller) (Variables|/Game/Core/Player/PC_Ingame.PC_Ingame_C|GetMineMax _playercontroller))
            (Variables|Mine|SetQuantityMine (+ (Variables|/Game/Core/Player/PC_Ingame.PC_Ingame_C|GetMine _playercontroller) (Variables|Mine|GetQuantityMine)))
            (Default|SetText _statuscontainerwidget (Variables|Stats|GetName) (Variables|Mine|GetQuantityMine))
            (Default|SetPercent _statuscontainerwidget (Variables|Mine|GetQuantityMine) (Variables|Stats|GetQuantityMax))
            (Default|IncrementMineralContainer _gamemode (Variables|Stats|GetName) (Variables|Mine|GetQuantityMine) (Variables|Stats|GetQuantityMax))
            (Variables|/Game/Core/Player/PC_Ingame.PC_Ingame_C|SetMine _playercontroller 0.0)
            (Default|DecrementMineralCollectPlayer _gamemode)
            (goto _label)))))
    (:NewEnumerator2
      (if (>= (Variables|Water|GetQuantityWater) (Variables|Stats|GetQuantityMax))
        (Variables|Water|SetQuantityWater (Variables|Stats|GetQuantityMax))
        (bind _output_get_2 (Variables|Water|SetbIsFullWater true))
        (Development|PrintString (Utilities|String|ToString(Boolean) _output_get_2))
        (goto _label)
        (elif (<= (Variables|/Game/Core/Player/PC_Ingame.PC_Ingame_C|GetWater _playercontroller) 0.0)
          (goto _label)
          (elif (< (Variables|/Game/Core/Player/PC_Ingame.PC_Ingame_C|GetWater _playercontroller) (Variables|/Game/Core/Player/PC_Ingame.PC_Ingame_C|GetWaterMax _playercontroller))
            (Variables|Water|SetQuantityWater (+ (Variables|/Game/Core/Player/PC_Ingame.PC_Ingame_C|GetWater _playercontroller) (Variables|Water|GetQuantityWater)))
            (Default|SetText _statuscontainerwidget (Variables|Stats|GetName) (Variables|Water|GetQuantityWater))
            (Default|SetPercent _statuscontainerwidget (Variables|Water|GetQuantityWater) (Variables|Stats|GetQuantityMax))
            (Default|IncrementWaterContainer _gamemode (Variables|Stats|GetName) (Variables|Water|GetQuantityWater) (Variables|Stats|GetQuantityMax))
            (Variables|/Game/Core/Player/PC_Ingame.PC_Ingame_C|SetWater _playercontroller 0.0)
            (Default|DecrementWaterCollectPlayer _gamemode)
            (goto _label)))))))

(event EventBeginPlay
  (bind _quantity (Variables|Stats|GetQuantity))
  (bind _gamemode (CallFunction|CastGameMode))
  (Variables|Reference|SetGameMode _gamemode)
  (bind _controller (CallFunction|CastController))
  (Variables|Reference|SetPlayerController _controller)
  (bind _character (CallFunction|CastCharacter))
  (Variables|Reference|SetCharacter _character)
  (bind _statuscontainerwidget (CallFunction|CastWidgetContainer (Variables|Default|GetStatus)))
  (bind _output_get (Variables|Reference|SetStatusContainerWidget _statuscontainerwidget))
  (Default|SetColorWidget _output_get (Variables|Stats|GetType))
  (Default|SetText _output_get (Variables|Stats|GetName) _quantity)
  (Default|SetPercent _output_get _quantity (Variables|Stats|GetQuantityMax)))

(event Collision|EventActorBeginOverlap
  (params (OtherActor :type Actor%20Object%20Reference))
  (bind _character (Variables|Reference|GetCharacter))
  (bind _widgetr (Variables|/Game/Core/Player/BP_Character.BP_Character_C|GetWidgetR _character))
  (bind _widgetl (Variables|/Game/Core/Player/BP_Character.BP_Character_C|GetWidgetL _character))
  (if (== OtherActor (Variables|Reference|GetCharacter))
    (bind _output_get (Variables|Stats|SetLocationMesh "0, 0,-70.000000"))
    (Transformation|SetRelativeLocation (Variables|Default|GetPlatformReservoirMesh) _output_get false false)
    (CallFunction|IncrementResourceContainer)
    (bind _returnvalue (Actor|GetActorOfClass "/Game/Core/Actor/Elevator/BP_Elevator.BP_Elevator_C"))
    (Variables|/Game/Core/Actor/Elevator/BP_Elevator.BP_Elevator_C|SetbDownActive _returnvalue true)
    (switch Utilities|FlowControl|Switch|SwitchonE_Type (Variables|Stats|GetType)
      (:NewEnumerator0
        (Rendering|SetVisibility _widgetr true false)
        (Utilities|FlowControl|Delay 0.2)
        (Rendering|SetVisibility _widgetr false false)
        (Utilities|FlowControl|Delay 0.2)
        (Rendering|SetVisibility _widgetr true false)
        (Utilities|FlowControl|Delay 0.2)
        (Rendering|SetVisibility _widgetr false false))
      (:NewEnumerator2
        (Rendering|SetVisibility _widgetl true false)
        (Utilities|FlowControl|Delay 0.2)
        (Rendering|SetVisibility _widgetl false false)
        (Utilities|FlowControl|Delay 0.2)
        (Rendering|SetVisibility _widgetl true false)
        (Utilities|FlowControl|Delay 0.2)
        (Rendering|SetVisibility _widgetl false false)))))

(event Collision|EventActorEndOverlap
  (params (OtherActor :type Actor%20Object%20Reference))
  (if (== OtherActor (Variables|Reference|GetCharacter))
    (bind _output_get (Variables|Stats|SetLocationMesh "0, 0,-60.000000"))
    (Transformation|SetRelativeLocation (Variables|Default|GetPlatformReservoirMesh) _output_get false false)))

(fn ConstructionScript
  ;[1 1 1] Box collision
  (bind _returnvalue (AddComponent|AddBoxComponent false))
  (Components|Box|SetBoxExtent _returnvalue (Variables|Stats|GetBoxExtent) true)
  (Transformation|SetRelativeLocation _returnvalue "0, 0,-50.000000" false false)
  ;[1 1 1] Static Mesh
  (bind _returnvalue_2 (AddComponent|AddStaticMeshComponent false))
  (bind _output_get (Variables|Default|SetPlatformReservoirMesh _returnvalue_2))
  (Transformation|SetWorldScale3D _output_get "1.000000,2.000000,0.200000")
  (Transformation|SetRelativeLocation _output_get (Variables|Stats|GetLocationMesh) false false))