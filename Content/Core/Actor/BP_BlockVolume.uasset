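; Blocking volume that penalizes the player and reverses a descending BP_Elevator on overlap.
; Caches game mode, controller, character and elevator on BeginPlay, with its box collision added in the construction script.
; Player overlap deducts health, updates the HUD, then after a short delay teleports the character above the elevator's ButtonDownUp.
; Elevator overlap during descent pauses its down timer and starts a looping timer that calls MoveUp.
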(event Custom|StartMoveUp
  (Default|MoveUp (Variables|Default|GetElevator)))

(event EventBeginPlay
  (bind _gamemode (CallFunction|CastGameMode))
  (Variables|Default|SetGame%20Mode _gamemode)
  (bind _controller (CallFunction|CastController))
  (Variables|Default|SetController _controller)
  (bind _character (CallFunction|CastCharacter))
  (Variables|Default|SetCharacter _character)
  (bind _returnvalue (Actor|GetActorOfClass "/Game/Core/Actor/Elevator/BP_Elevator.BP_Elevator_C"))
  (Variables|Default|SetElevator _returnvalue))

(event Collision|EventActorBeginOverlap
  (params (OtherActor :type Actor%20Object%20Reference))
  (bind _elevator (Variables|Default|GetElevator))
  (bind _elevator_2 (Variables|Default|GetElevator))
  (bind _controller (Variables|Default|GetController))
  (bind _buttondownup (Variables|/Game/Core/Actor/Elevator/BP_Elevator.BP_Elevator_C|GetButtonDownUp _elevator))
  (bind _playerstats (Variables|/Game/Core/Player/PC_Ingame.PC_Ingame_C|GetPlayerStats _controller))
  (bind _returnvalue (Transformation|GetWorldLocation _buttondownup))
  (if (== OtherActor (Variables|Default|GetCharacter))
    (bind _structout (Utilities|Struct|SetmembersinS_PlayerStats _playerstats (- (Utilities|Struct|BreakS_PlayerStats _playerstats) 1e+01)))
    (Default|SetPlayerHealth (Variables|/Game/Core/Settings/GM_Main.GM_Main_C|GetUI_Player (Variables|Default|GetGame%20Mode)) (Utilities|Struct|BreakS_PlayerStats _structout))
    (Utilities|FlowControl|Delay 1.0)
    (Transformation|Teleport (Variables|Default|GetCharacter) (Math|Vector|MakeVector (.x _returnvalue) (.y _returnvalue) (+ (.z _returnvalue) 75.0)) "0, 0, 0")
    (else
      (Utilities|FlowControl|Sequence
        (:then_0
          (bind _returnvalue_2 (Actor|GetActorOfClass "/Game/Core/Actor/Water/BP_Water.BP_Water_C"))
          (if (not (== _returnvalue_2 OtherActor))
            (bind _returnvalue_3 (Actor|GetActorOfClass "/Game/Core/Actor/Elevator/BP_Elevator.BP_Elevator_C" :!label _label))
            (if (== _returnvalue_3 OtherActor)
              (if (Variables|/Game/Core/Actor/Elevator/BP_Elevator.BP_Elevator_C|GetbDownActive _elevator_2)
                (Utilities|Time|PauseTimerbyHandle (Variables|/Game/Core/Actor/Elevator/BP_Elevator.BP_Elevator_C|GetTimerDown _elevator_2))
                (Variables|/Game/Core/Actor/Elevator/BP_Elevator.BP_Elevator_C|SetbDownActive _elevator_2 false)
                (bind _returnvalue_4 (Utilities|Time|SetTimerbyEvent (delegate Custom|StartMoveUp) 0.01 true))
                (Variables|Default|SetTimerMoveUp _returnvalue_4)))))
        (:then_1
          (goto _label))))))

(fn ConstructionScript
  (bind _returnvalue (AddComponent|AddBoxComponent false))
  (Variables|Default|SetBoxCollision _returnvalue))