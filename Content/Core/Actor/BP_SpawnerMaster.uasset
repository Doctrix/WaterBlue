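; BP_SpawnerMaster is a configurable spawner for mineral (BP_Mine), enemy or water actors, selected by its Type.
; The construction script adds a box sized by BoxExtent, and spawn functions place actors at random points inside it.
; Mineral and Enemy types start looping timers on BeginPlay, while Water starts one after a character overlap and short delay.
; Each timer's interval is randomized once, when it is set.
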(event Collision|EventActorBeginOverlap
  (params (OtherActor :type Actor%20Object%20Reference))
  ;[1 1 1] Faire tomber Water au contact collision
  (bind _character (CallFunction|CastCharacter))
  (if (== _character OtherActor)
    (switch Utilities|FlowControl|Switch|SwitchonE_Type (Variables|Default|GetType)
      (:NewEnumerator2
        (Utilities|FlowControl|Delay 2.0)
        (Utilities|Time|SetTimerbyEvent (EventDispatchers|CreateEvent :!event SpawnWater) (Math|Random|RandomFloatinRange 1.0 3.0) true)))))

(event EventBeginPlay
  (switch Utilities|FlowControl|Switch|SwitchonE_Type (Variables|Default|GetType)
    (:NewEnumerator0
      (Utilities|Time|SetTimerbyEvent (EventDispatchers|CreateEvent :!event SpawnItem) (Math|Random|RandomFloatinRange 1.0 3.0) true))
    (:NewEnumerator1
      (Utilities|Time|SetTimerbyEvent (EventDispatchers|CreateEvent :!event SpawnEnemy) (Math|Random|RandomFloatinRange 0.2 1.5) true))))

(fn ConstructionScript
  (bind _returnvalue (AddComponent|AddBoxComponent false))
  (bind _output_get (Variables|Default|SetBoxCollision _returnvalue))
  (Components|Box|SetBoxExtent _output_get (Variables|Default|GetBoxExtent) true))

(fn SpawnItem
  (bind _boxcollision (Variables|Default|GetBoxCollision))
  (Game|SpawnActorfromClass "/Game/Core/Item/Mineral/BP_Mine.BP_Mine_C" (Math|Transform|MakeTransform (Math|Random|RandomPointinBoundingBox (Transformation|GetWorldLocation _boxcollision) (Variables|/Script/Engine.BoxComponent|GetBoxExtent _boxcollision)) "0, 0, 0" "1,1,1") "Undefined" 0 0)
  (return))

(fn SpawnEnemy
  (bind _boxcollision (Variables|Default|GetBoxCollision))
  (Game|SpawnActorfromClass "/Game/Core/Enemy/BP_Enemy.BP_Enemy_C" (Math|Transform|MakeTransform (Math|Random|RandomPointinBoundingBox (Transformation|GetWorldLocation _boxcollision) (Variables|/Script/Engine.BoxComponent|GetBoxExtent _boxcollision)) (Transformation|GetWorldRotation _boxcollision) "1,1,1") "Undefined" 0 0)
  (return))

(fn SpawnWater
  (bind _boxcollision (Variables|Default|GetBoxCollision))
  (Game|SpawnActorfromClass "/Game/Core/Item/Water/BP_Water.BP_Water_C" (Math|Transform|MakeTransform (Math|Random|RandomPointinBoundingBox (Transformation|GetWorldLocation _boxcollision) (Variables|/Script/Engine.BoxComponent|GetBoxExtent _boxcollision)) "0, 0, 0" "1,1,1") "Undefined" 0 0)
  (return))