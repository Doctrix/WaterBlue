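; Elevator platform that the player character moves up, down, left or right by standing on overlap buttons.
; Buttons run looping timers; the up/down one also toggles two trap pieces and picks direction from DownActive, while side buttons toggle lights.
; Move events play timelines that offset the mesh and cache its world position, only once GM_Main's StartGame is true.
; Construction script adds a child actor and, if it is a BP_SpawnerMaster, resizes its collision box.
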(event OnComponentBeginOverlap(ButtonLeft)
  (params (OverlappedComponent :type Primitive%20Component%20Object%20Reference) (OtherActor :type Actor%20Object%20Reference) (OtherComp :type Primitive%20Component%20Object%20Reference) (OtherBodyIndex :type Integer) (bFromSweep :type Boolean) (SweepResult :type Hit%20Result%20Structure%20%28by%20ref%29))
  ;[1 1 1] Button Gauche
  (if (== OtherActor (Variables|Reference|GetCharacter))
    (Rendering|SetVisibility (Variables|Default|GetPointLightLeft) true false)
    (bind _returnvalue (Utilities|Time|SetTimerbyEvent (EventDispatchers|CreateEvent :!event Custom|MoveLeft) 0.01 true))
    (Variables|Event|SetTimerLeft _returnvalue)))

(event OnComponentEndOverlap(ButtonLeft)
  (params (OverlappedComponent :type Primitive%20Component%20Object%20Reference) (OtherActor :type Actor%20Object%20Reference) (OtherComp :type Primitive%20Component%20Object%20Reference) (OtherBodyIndex :type Integer))
  ;[1 1 1] Button Gauche
  (if (== OtherActor (Variables|Reference|GetCharacter))
    (Rendering|SetVisibility (Variables|Default|GetPointLightLeft) false false)
    (Utilities|Time|ClearandInvalidateTimerbyHandle (Variables|Event|GetTimerLeft))))

(event OnComponentBeginOverlap(ButtonRight)
  (params (OverlappedComponent :type Primitive%20Component%20Object%20Reference) (OtherActor :type Actor%20Object%20Reference) (OtherComp :type Primitive%20Component%20Object%20Reference) (OtherBodyIndex :type Integer) (bFromSweep :type Boolean) (SweepResult :type Hit%20Result%20Structure%20%28by%20ref%29))
  ;[1 1 1] Button droite
  (if (== OtherActor (Variables|Reference|GetCharacter))
    (Rendering|SetVisibility (Variables|Default|GetPointLightRight) true false)
    (bind _returnvalue (Utilities|Time|SetTimerbyEvent (EventDispatchers|CreateEvent :!event Custom|MoveRight) 0.01 true))
    (Variables|Event|SetTimerRight _returnvalue)))

(event OnComponentEndOverlap(ButtonRight)
  (params (OverlappedComponent :type Primitive%20Component%20Object%20Reference) (OtherActor :type Actor%20Object%20Reference) (OtherComp :type Primitive%20Component%20Object%20Reference) (OtherBodyIndex :type Integer))
  ;[1 1 1] Button droite
  (if (== OtherActor (Variables|Reference|GetCharacter))
    (Rendering|SetVisibility (Variables|Default|GetPointLightRight) false false)
    (Utilities|Time|ClearandInvalidateTimerbyHandle (Variables|Event|GetTimerRight))))

(event OnComponentBeginOverlap(ButtonDownUp)
  (params (OverlappedComponent :type Primitive%20Component%20Object%20Reference) (OtherActor :type Actor%20Object%20Reference) (OtherComp :type Primitive%20Component%20Object%20Reference) (OtherBodyIndex :type Integer) (bFromSweep :type Boolean) (SweepResult :type Hit%20Result%20Structure%20%28by%20ref%29))
  ;[1 1 1] Button Down
  (if (== OtherActor (Variables|Reference|GetCharacter))
    (Transformation|SetRelativeLocation (Variables|Default|GetBoxTrapeLeft) (Variables|Default|GetPosTrapeLeftOpen) false false)
    (Transformation|SetRelativeLocation (Variables|Default|GetBoxTrapeRight) (Variables|Default|GetPosTrapRightOpen) false false)
    (if (Variables|Boolean|GetbDownActive)
      (bind _returnvalue (Utilities|Time|SetTimerbyEvent (delegate Custom|StartDown) 0.01 true))
      (Variables|Event|SetTimerDown _returnvalue)
      (else
        (bind _returnvalue_2 (Utilities|Time|SetTimerbyEvent (delegate Custom|StartUp) 0.01 true))
        (Variables|Event|SetTimerUp _returnvalue_2)))))

(event OnComponentEndOverlap(ButtonDownUp)
  (params (OverlappedComponent :type Primitive%20Component%20Object%20Reference) (OtherActor :type Actor%20Object%20Reference) (OtherComp :type Primitive%20Component%20Object%20Reference) (OtherBodyIndex :type Integer))
  ;[1 1 1] Button Down
  (if (== OtherActor (Variables|Reference|GetCharacter))
    (Transformation|SetRelativeLocation (Variables|Default|GetBoxTrapeLeft) (Variables|Default|GetPosTrapLeftClose) false false)
    (Transformation|SetRelativeLocation (Variables|Default|GetBoxTrapeRight) (Variables|Default|GetPosTrapRightClose) false false)
    (if (Variables|Boolean|GetbDownActive)
      (Utilities|Time|PauseTimerbyHandle (Variables|Event|GetTimerDown))
      (else
        (Utilities|Time|PauseTimerbyHandle (Variables|Event|GetTimerUp))))))

(event Custom|MoveUp
  ;[1 1 1] Move up elevator
  (Utilities|StartGameTrue
    (:true
      (bind _up (Timeline|Up Play)
        (:Update
          (Class|SceneComponent|AddLocalTransform (Variables|Debug|GetStaticMeshComponent) (Math|Transform|MakeTransform (Math|Vector|MakeVector 0.0 0.0 _up) "0, 0, 0" (Variables|Default|GetScalePlatform)) false false)
          ;[1 1 1] Move Down elevator
          (CallFunction|PosRef))))))

(event Custom|MoveRight
  ;[1 1 1] Move Right Elevator
  (Utilities|StartGameTrue
    (:true
      (bind _speed (Timeline|Right Play)
        (:Update
          (Class|SceneComponent|AddLocalTransform (Variables|Debug|GetStaticMeshComponent) (Math|Transform|MakeTransform (Math|Vector|MakeVector 0.0 _speed 0.0) "0, 0, 0" (Variables|Default|GetScalePlatform)) false false)
          ;[1 1 1] Move Down elevator
          (CallFunction|PosRef))))))

(event Custom|MoveLeft
  ;[1 1 1] Move Left Elevator
  (Utilities|StartGameTrue
    (:true
      (bind _speed (Timeline|Left Play)
        (:Update
          (Class|SceneComponent|AddLocalTransform (Variables|Debug|GetStaticMeshComponent) (Math|Transform|MakeTransform (Math|Vector|MakeVector 0.0 _speed 0.0) "0, 0, 0" (Variables|Default|GetScalePlatform)) false false)
          ;[1 1 1] Move Down elevator
          (CallFunction|PosRef))))))

(event Custom|StartUp
  ;[1 1 1] Button Down
  (CallFunction|MoveUp))

(event Custom|StopUp
  ;[1 1 1] Move up elevator
  (bind _up (Timeline|Up Stop)
    (:Update
      (Class|SceneComponent|AddLocalTransform (Variables|Debug|GetStaticMeshComponent) (Math|Transform|MakeTransform (Math|Vector|MakeVector 0.0 0.0 _up) "0, 0, 0" (Variables|Default|GetScalePlatform)) false false)
      ;[1 1 1] Move Down elevator
      (CallFunction|PosRef))))

(event Custom|StopLeft
  ;[1 1 1] Move Left Elevator
  (bind _speed (Timeline|Left Stop)
    (:Update
      (Class|SceneComponent|AddLocalTransform (Variables|Debug|GetStaticMeshComponent) (Math|Transform|MakeTransform (Math|Vector|MakeVector 0.0 _speed 0.0) "0, 0, 0" (Variables|Default|GetScalePlatform)) false false)
      ;[1 1 1] Move Down elevator
      (CallFunction|PosRef))))

(event Custom|StopRight
  ;[1 1 1] Move Right Elevator
  (bind _speed (Timeline|Right Stop)
    (:Update
      (Class|SceneComponent|AddLocalTransform (Variables|Debug|GetStaticMeshComponent) (Math|Transform|MakeTransform (Math|Vector|MakeVector 0.0 _speed 0.0) "0, 0, 0" (Variables|Default|GetScalePlatform)) false false)
      ;[1 1 1] Move Down elevator
      (CallFunction|PosRef))))

(event Custom|MoveDown
  ;[1 1 1] Move Down elevator
  (Utilities|StartGameTrue
    (:true
      (bind _speed (Timeline|Down Play)
        (:Update
          (Class|SceneComponent|AddLocalTransform (Variables|Debug|GetStaticMeshComponent) (Math|Transform|MakeTransform (Math|Vector|MakeVector 0.0 0.0 _speed) "0, 0, 0" (Variables|Default|GetScalePlatform)) false false)
          (CallFunction|PosRef))))))

(event Custom|StopDown
  ;[1 1 1] Move Down elevator
  (bind _speed (Timeline|Down Stop)
    (:Update
      (Class|SceneComponent|AddLocalTransform (Variables|Debug|GetStaticMeshComponent) (Math|Transform|MakeTransform (Math|Vector|MakeVector 0.0 0.0 _speed) "0, 0, 0" (Variables|Default|GetScalePlatform)) false false)
      (CallFunction|PosRef))))

(event Custom|StartDown
  ;[1 1 1] Button Down
  (CallFunction|MoveDown))

(event EventBeginPlay
  (bind _character (CallFunction|CastCharacter))
  (Variables|Reference|SetCharacter _character)
  (CallFunction|PosRef))

(fn ConstructionScript
  (bind _returnvalue (AddComponent|AddChildActorComponent false))
  (bind _asbp_spawner_master (Utilities|Casting|CastToBP_SpawnerMaster (Variables|/Script/Engine.ChildActorComponent|GetChildActor _returnvalue)))
  (Components|Box|SetBoxExtent (Variables|/Game/Core/Actor/BP_SpawnerMaster.BP_SpawnerMaster_C|GetBoxCollision _asbp_spawner_master) "32.000000,200.000000,300.000000" true))

(fn PosRef
  (bind _staticmeshcomponent (Variables|Debug|GetStaticMeshComponent))
  (bind _returnvalue (Transformation|GetWorldLocation _staticmeshcomponent))
  ;[1 1 1] Position elevator
  (Variables|Position|SetPosX (.x _returnvalue))
  (Variables|Position|SetPosY (.y _returnvalue))
  (Variables|Position|SetPosZ (.z _returnvalue))
  (return))