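; BP_Elevator is a platform the player character drives by standing on button triggers, moving vertically or sideways once GM_Main's StartGame is set.
; Button overlaps start looping timers, paused or cleared on exit; DownActive selects up or down, and the left and right buttons also light up.
; Move events play timelines that offset the mesh by local transforms without sweep, then PosRef caches its world position.
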(event OnComponentBeginOverlap(ButtonLeft)
  (params (OverlappedComponent :type Primitive%20Component%20Object%20Reference) (OtherActor :type Actor%20Object%20Reference) (OtherComp :type Primitive%20Component%20Object%20Reference) (OtherBodyIndex :type Integer) (bFromSweep :type Boolean) (SweepResult :type Hit%20Result%20Structure%20%28by%20ref%29))
  ;[1 1 1] Button Gauche
  (if (== OtherActor (Variables|Reference|GetCharacter))
    (Rendering|SetVisibility (Variables|Default|GetPointLightLeft) true false)
    (bind _returnvalue (Utilities|Time|SetTimerbyEvent (EventDispatchers|CreateEvent :!event Custom|MoveLeft) 0.01 true))
    (Variables|Event|SetTimerLeft _returnvalue)))

(event OnComponentEndOverlap(ButtonLeft)
  (params (OverlappedComponent :type Primitive%20Component%20Object%20Reference) (OtherActor :type Actor%20Object%20Reference) (OtherComp :type Primitive%20Component%20Object%20Reference) (OtherBodyIndex :type Integer))
  ;[1 1 1] Button Gauche
  (if (== OtherActor (Variables|Reference|GetCharacter))
    (Rendering|SetVisibility (Variables|Default|GetPointLightLeft) false false)
    (Utilities|Time|ClearandInvalidateTimerbyHandle (Variables|Event|GetTimerLeft))))

(event OnComponentBeginOverlap(ButtonRight)
  (params (OverlappedComponent :type Primitive%20Component%20Object%20Reference) (OtherActor :type Actor%20Object%20Reference) (OtherComp :type Primitive%20Component%20Object%20Reference) (OtherBodyIndex :type Integer) (bFromSweep :type Boolean) (SweepResult :type Hit%20Result%20Structure%20%28by%20ref%29))
  ;[1 1 1] Button droite
  (if (== OtherActor (Variables|Reference|GetCharacter))
    (Rendering|SetVisibility (Variables|Default|GetPointLightRight) true false)
    (bind _returnvalue (Utilities|Time|SetTimerbyEvent (EventDispatchers|CreateEvent :!event Custom|MoveRight) 0.01 true))
    (Variables|Event|SetTimerRight _returnvalue)))

(event OnComponentEndOverlap(ButtonRight)
  (params (OverlappedComponent :type Primitive%20Component%20Object%20Reference) (OtherActor :type Actor%20Object%20Reference) (OtherComp :type Primitive%20Component%20Object%20Reference) (OtherBodyIndex :type Integer))
  ;[1 1 1] Button droite
  (if (== OtherActor (Variables|Reference|GetCharacter))
    (Rendering|SetVisibility (Variables|Default|GetPointLightRight) false false)
    (Utilities|Time|ClearandInvalidateTimerbyHandle (Variables|Event|GetTimerRight))))

(event OnComponentBeginOverlap(ButtonDownUp)
  (params (OverlappedComponent :type Primitive%20Component%20Object%20Reference) (OtherActor :type Actor%20Object%20Reference) (OtherComp :type Primitive%20Component%20Object%20Reference) (OtherBodyIndex :type Integer) (bFromSweep :type Boolean) (SweepResult :type Hit%20Result%20Structure%20%28by%20ref%29))
  ;[1 1 1] Button Down
  (if (== OtherActor (Variables|Reference|GetCharacter))
    (if (Variables|Default|GetbDownActive)
      (bind _returnvalue (Utilities|Time|SetTimerbyEvent (delegate Custom|CustomEvent_1) 0.01 true))
      (Variables|Default|SetNewVar_0 _returnvalue)
      (else
        (bind _returnvalue_2 (Utilities|Time|SetTimerbyEvent (delegate Custom|CustomEvent_0) 0.01 true))
        (Variables|Default|SetNewVar_1 _returnvalue_2)))))

(event OnComponentEndOverlap(ButtonDownUp)
  (params (OverlappedComponent :type Primitive%20Component%20Object%20Reference) (OtherActor :type Actor%20Object%20Reference) (OtherComp :type Primitive%20Component%20Object%20Reference) (OtherBodyIndex :type Integer))
  ;[1 1 1] Button Down
  (if (== OtherActor (Variables|Reference|GetCharacter))
    (if (Variables|Default|GetbDownActive)
      (Utilities|Time|PauseTimerbyHandle (Variables|Default|GetNewVar_0))
      (else
        (Utilities|Time|PauseTimerbyHandle (Variables|Default|GetNewVar_1))))))

(event Custom|MoveUp
  ;[1 1 1] Move Down elevator
  (Utilities|StartGameTrue
    (:true
      (bind _up (Timeline|Up Play)
        (:Update
          (Class|SceneComponent|AddLocalTransform (Variables|Debug|GetStaticMeshComponent) (Math|Transform|MakeTransform (Math|Vector|MakeVector 0.0 0.0 _up) "0, 0, 0" (Variables|Default|GetScalePlatform)) false false)
          (CallFunction|PosRef))))))

(event Custom|MoveRight
  ;[1 1 1] Move Right Elevator
  (Utilities|StartGameTrue
    (:true
      (bind _speed (Timeline|Right Play)
        (:Update
          (Class|SceneComponent|AddLocalTransform (Variables|Debug|GetStaticMeshComponent) (Math|Transform|MakeTransform (Math|Vector|MakeVector 0.0 _speed 0.0) "0, 0, 0" (Variables|Default|GetScalePlatform)) false false)
          (CallFunction|PosRef))))))

(event Custom|MoveLeft
  ;[1 1 1] Move Left Elevator
  (Utilities|StartGameTrue
    (:true
      (bind _speed (Timeline|Left Play)
        (:Update
          (Class|SceneComponent|AddLocalTransform (Variables|Debug|GetStaticMeshComponent) (Math|Transform|MakeTransform (Math|Vector|MakeVector 0.0 _speed 0.0) "0, 0, 0" (Variables|Default|GetScalePlatform)) false false)
          (CallFunction|PosRef))))))

(event Custom|CustomEvent_0
  ;[1 1 1] Button Down
  (CallFunction|MoveUp))

(event Custom|StopUp
  ;[1 1 1] Move Down elevator
  (bind _up (Timeline|Up Stop)
    (:Update
      (Class|SceneComponent|AddLocalTransform (Variables|Debug|GetStaticMeshComponent) (Math|Transform|MakeTransform (Math|Vector|MakeVector 0.0 0.0 _up) "0, 0, 0" (Variables|Default|GetScalePlatform)) false false)
      (CallFunction|PosRef))))

(event Custom|StopLeft
  ;[1 1 1] Move Left Elevator
  (bind _speed (Timeline|Left Stop)
    (:Update
      (Class|SceneComponent|AddLocalTransform (Variables|Debug|GetStaticMeshComponent) (Math|Transform|MakeTransform (Math|Vector|MakeVector 0.0 _speed 0.0) "0, 0, 0" (Variables|Default|GetScalePlatform)) false false)
      (CallFunction|PosRef))))

(event Custom|StopRight
  ;[1 1 1] Move Right Elevator
  (bind _speed (Timeline|Right Stop)
    (:Update
      (Class|SceneComponent|AddLocalTransform (Variables|Debug|GetStaticMeshComponent) (Math|Transform|MakeTransform (Math|Vector|MakeVector 0.0 _speed 0.0) "0, 0, 0" (Variables|Default|GetScalePlatform)) false false)
      (CallFunction|PosRef))))

(event Custom|MoveDown
  ;[1 1 1] Move Down elevator
  (Utilities|StartGameTrue
    (:true
      (bind _speed (Timeline|Down Play)
        (:Update
          (Class|SceneComponent|AddLocalTransform (Variables|Debug|GetStaticMeshComponent) (Math|Transform|MakeTransform (Math|Vector|MakeVector 0.0 0.0 _speed) "0, 0, 0" (Variables|Default|GetScalePlatform)) false false)
          (CallFunction|PosRef))))))

(event Custom|StopDown
  ;[1 1 1] Move Down elevator
  (bind _speed (Timeline|Down Stop)
    (:Update
      (Class|SceneComponent|AddLocalTransform (Variables|Debug|GetStaticMeshComponent) (Math|Transform|MakeTransform (Math|Vector|MakeVector 0.0 0.0 _speed) "0, 0, 0" (Variables|Default|GetScalePlatform)) false false)
      (CallFunction|PosRef))))

(event Custom|CustomEvent_1
  (CallFunction|MoveDown))

(event EventBeginPlay
  (bind _character (CallFunction|CastCharacter))
  (Variables|Reference|SetCharacter _character)
  (CallFunction|PosRef))

(fn ConstructionScript)

(fn PosRef
  (bind _staticmeshcomponent (Variables|Debug|GetStaticMeshComponent))
  (bind _returnvalue (Transformation|GetWorldLocation _staticmeshcomponent))
  ;[1 1 1] Position elevator
  (Variables|Default|SetPosX (.x _returnvalue))
  (Variables|Default|SetPosY (.y _returnvalue))
  (Variables|Default|SetPosZ (.z _returnvalue))
  (return))