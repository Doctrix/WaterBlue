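; Base resource container where the player deposits Mineral or Water by stepping on a platform built in the construction script.
; Overlap sinks the platform, activates BP_Elevator's DownActive and blinks the character widget for that type.
; A full player Mine value is added to Quantity and reported through GameMode; only the Mineral branch resets Mine.
; BeginPlay initializes the status widget with type color, name and fill level.
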(event Custom|IncrementResourceContainer
  (bind _playercontroller (Variables|Reference|GetPlayerController))
  (bind _gamemode (Variables|Reference|GetGameMode))
  (bind _playercontroller_2 (Variables|Reference|GetPlayerController))
  (switch Utilities|FlowControl|Switch|SwitchonE_Type (Variables|Default|GetType)
    (:NewEnumerator0
      (if (not (== (Variables|/Game/Core/Player/PC_Ingame.PC_Ingame_C|GetMine _playercontroller) 0.0))
        (if (not (< (Variables|/Game/Core/Player/PC_Ingame.PC_Ingame_C|GetMine _playercontroller) (Variables|/Game/Core/Player/PC_Ingame.PC_Ingame_C|GetMineMax _playercontroller)))
          (Variables|Default|SetQuantity (+ (Variables|/Game/Core/Player/PC_Ingame.PC_Ingame_C|GetMine _playercontroller) (Variables|Default|GetQuantity)))
          (Default|IncrementMineralContainer _gamemode (Variables|Default|GetName) (Variables|Default|GetQuantity) (Variables|Default|GetQuantityMax))
          (Variables|/Game/Core/Player/PC_Ingame.PC_Ingame_C|SetMine _playercontroller 0.0)
          (Default|DecrementMineralCollectPlayer _gamemode))))
    (:NewEnumerator2
      (if (not (== (Variables|/Game/Core/Player/PC_Ingame.PC_Ingame_C|GetMine _playercontroller_2) 0.0))
        (if (not (< (Variables|/Game/Core/Player/PC_Ingame.PC_Ingame_C|GetMine _playercontroller_2) (Variables|/Game/Core/Player/PC_Ingame.PC_Ingame_C|GetMineMax _playercontroller_2)))
          (Variables|Default|SetQuantity (+ (Variables|/Game/Core/Player/PC_Ingame.PC_Ingame_C|GetMine _playercontroller_2) (Variables|Default|GetQuantity)))
          (Default|IncrementWaterContainer _gamemode (Variables|Default|GetName) (Variables|Default|GetQuantity) (Variables|Default|GetQuantityMax))
          (Default|DecrementWaterCollectPlayer _gamemode))))))

(event EventBeginPlay
  (bind _quantity (Variables|Default|GetQuantity))
  (bind _gamemode (CallFunction|CastGameMode))
  (Variables|Reference|SetGameMode _gamemode)
  (bind _controller (CallFunction|CastController))
  (Variables|Reference|SetPlayerController _controller)
  (bind _character (CallFunction|CastCharacter))
  (Variables|Reference|SetCharacter _character)
  (bind _statuscontainerwidget (CallFunction|CastWidgetContainer (Variables|Default|GetStatus)))
  (bind _output_get (Variables|Reference|SetStatusContainerWidget _statuscontainerwidget))
  (Default|SetColorWidget _output_get (Variables|Default|GetType))
  (Default|SetText _output_get (Variables|Default|GetName) _quantity)
  (Default|SetPercent _output_get _quantity (Variables|Default|GetQuantityMax)))

(event Collision|EventActorBeginOverlap
  (params (OtherActor :type Actor%20Object%20Reference))
  (bind _character (Variables|Reference|GetCharacter))
  (bind _widgetr (Variables|/Game/Core/Player/BP_Character.BP_Character_C|GetWidgetR _character))
  (bind _widgetl (Variables|/Game/Core/Player/BP_Character.BP_Character_C|GetWidgetL _character))
  (if (== OtherActor (Variables|Reference|GetCharacter))
    (bind _output_get (Variables|Default|SetLocationMesh "0, 0,-70.000000"))
    (Transformation|SetRelativeLocation (Variables|Default|GetPlatformReservoirMesh) _output_get false false)
    (CallFunction|IncrementResourceContainer)
    (bind _returnvalue (Actor|GetActorOfClass "/Game/Core/Elevator/BP_Elevator.BP_Elevator_C"))
    (Variables|/Game/Core/Elevator/BP_Elevator.BP_Elevator_C|SetbDownActive _returnvalue true)
    (switch Utilities|FlowControl|Switch|SwitchonE_Type (Variables|Default|GetType)
      (:NewEnumerator0
        (Rendering|SetVisibility _widgetr true false)
        (Utilities|FlowControl|Delay 0.2)
        (Rendering|SetVisibility _widgetr false false)
        (Utilities|FlowControl|Delay 0.2)
        (Rendering|SetVisibility _widgetr true false)
        (Utilities|FlowControl|Delay 0.2)
        (Rendering|SetVisibility _widgetr false false))
      (:NewEnumerator2
        (Rendering|SetVisibility _widgetl true false)
        (Utilities|FlowControl|Delay 0.2)
        (Rendering|SetVisibility _widgetl false false)
        (Utilities|FlowControl|Delay 0.2)
        (Rendering|SetVisibility _widgetl true false)
        (Utilities|FlowControl|Delay 0.2)
        (Rendering|SetVisibility _widgetl false false)))))

(event Collision|EventActorEndOverlap
  (params (OtherActor :type Actor%20Object%20Reference))
  (if (== OtherActor (Variables|Reference|GetCharacter))
    (bind _output_get (Variables|Default|SetLocationMesh "0, 0,-60.000000"))
    (Transformation|SetRelativeLocation (Variables|Default|GetPlatformReservoirMesh) _output_get false false)))

(fn ConstructionScript
  (bind _returnvalue (AddComponent|AddBoxComponent false))
  (Components|Box|SetBoxExtent _returnvalue (Variables|Default|GetBoxExtent) true)
  (Transformation|SetRelativeLocation _returnvalue "0, 0,-56.000000" false false)
  (bind _returnvalue_2 (AddComponent|AddStaticMeshComponent false))
  (bind _output_get (Variables|Default|SetPlatformReservoirMesh _returnvalue_2))
  (Transformation|SetWorldScale3D _output_get "1.000000,2.000000,0.200000")
  (Transformation|SetRelativeLocation _returnvalue_2 (Variables|Default|GetLocationMesh) false false))