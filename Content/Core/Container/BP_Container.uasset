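; Storage container for minerals or water that takes deposits from the player character standing on its pressure-plate-like platform.
; The construction script builds a trigger box and platform mesh, and BeginPlay initializes the status widget.
; On overlap, the platform sinks and each non-empty mineral or water inventory triggers a type-based transfer through GameMode if capacity remains.
; Minerals update the stored quantity, while water only calls the player decrement; leaving raises the platform.
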(event EventBeginPlay
  (bind _informations (Variables|Default|GetInformations))
  (bind (_type _quantity _quantitymax) (Utilities|Struct|BreakS_Container _informations))
  (bind _gamemode (CallFunction|CastGameMode))
  (Variables|Reference|SetGameMode _gamemode)
  (bind _controller (CallFunction|CastController))
  (Variables|Reference|SetPlayerController _controller)
  (bind _character (CallFunction|CastCharacter))
  (Variables|Reference|SetCharacter _character)
  (bind _statuscontainerwidget (CallFunction|CastWidgetContainer (Variables|Default|GetStatus)))
  (bind _output_get (Variables|Reference|SetStatusContainerWidget _statuscontainerwidget))
  (Default|SetQuantity _output_get _type _quantity _quantitymax))

(event Collision|EventActorBeginOverlap
  (params (OtherActor :type Actor%20Object%20Reference))
  (bind _gamemode (Variables|Reference|GetGameMode))
  (bind _informations (Variables|Default|GetInformations))
  (bind _playercontroller (Variables|Reference|GetPlayerController))
  (bind (_type _quantity _quantitymax _isfull) (Utilities|Struct|BreakS_Container _informations))
  (bind _ac_inventory (Variables|/Game/Core/Player/PC_Ingame.PC_Ingame_C|GetAC_Inventory _playercontroller))
  (bind _returnvalue (< _quantity _quantitymax))
  (bind _returnvalue_2 (not _isfull))
  (bind _returnvalue_3 (and _returnvalue _returnvalue_2))
  (if (== OtherActor (Variables|Reference|GetCharacter))
    (bind _output_get (Variables|Default|SetLocationMesh "0, 0,-70.000000"))
    (Transformation|SetRelativeLocation (Variables|Default|GetPlatformReservoirMesh) _output_get false false)
    (Utilities|FlowControl|Sequence
      (:then_0
        (if (not (== (Variables|/Game/Core/Player/AC_Inventory.AC_Inventory_C|GetQuantityMineralsCollected _ac_inventory) 0.0))
          (switch Utilities|FlowControl|Switch|SwitchonE_Type _type :!label _label
            (:NewEnumerator0
              (if _returnvalue_3
                (bind _quantitytotal (Default|IncrementMineralContainer _gamemode _quantity))
                (bind _structout (Utilities|Struct|SetmembersinS_Container (Variables|Default|GetInformations) _quantitytotal))
                (Development|PrintString (Utilities|String|ToString(Float) (Utilities|Struct|BreakS_Container _structout)))
                (Default|DecrementMineralCollectPlayer _gamemode)))
            (:NewEnumerator2
              (if _returnvalue_3
                (Default|DecrementWaterCollectPlayer _gamemode _quantity))))))
      (:then_1
        (if (not (== (Variables|/Game/Core/Player/AC_Inventory.AC_Inventory_C|GetQuantityWaterCollected _ac_inventory) 0.0))
          (goto _label))))))

(event Collision|EventActorEndOverlap
  (params (OtherActor :type Actor%20Object%20Reference))
  (if (== OtherActor (Variables|Reference|GetCharacter))
    (bind _output_get (Variables|Default|SetLocationMesh "0, 0,-60.000000"))
    (Transformation|SetRelativeLocation (Variables|Default|GetPlatformReservoirMesh) _output_get false false)))

(fn ConstructionScript
  (bind _returnvalue (AddComponent|AddBoxComponent false))
  (Components|Box|SetBoxExtent _returnvalue (Variables|Default|GetBoxExtent) true)
  (Transformation|SetRelativeLocation _returnvalue "0, 0,-56.000000" false false)
  (bind _returnvalue_2 (AddComponent|AddStaticMeshComponent false))
  (bind _output_get (Variables|Default|SetPlatformReservoirMesh _returnvalue_2))
  (Transformation|SetWorldScale3D _output_get "1.000000,2.000000,0.200000")
  (Transformation|SetRelativeLocation _returnvalue_2 (Variables|Default|GetLocationMesh) false false))