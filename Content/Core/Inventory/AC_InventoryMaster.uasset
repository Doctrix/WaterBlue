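; AC_InventoryMaster is an inventory component that stores items as SInventory entries in a slot-based array.
; On BeginPlay, PrepareInventory resizes the array to NumberSlots.
; AddToInventory finds the first entry matching an empty-name, default-type struct and overwrites it with the new content.
; It always returns true, with no check for a failed search when no empty slot exists.
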(event EventBeginPlay
  (CallFunction|PrepareInventory))

(event EventTick
  (params (DeltaSeconds :type Float%20%28single-precision%29)))

(fn AddtoInventory
  (params (ContentToAdd :type S%20Inventory%20Structure))
  (bind _inventory (Variables|Default|GetInventory))
  (Utilities|Array|SetArrayElem _inventory (Utilities|Array|FindItem _inventory (Utilities|Struct|MakeS_Inventory "" "NewEnumerator0")) ContentToAdd)
  (return true))

(fn PrepareInventory
  (Utilities|Array|Resize (Variables|Default|GetInventory) (Variables|Default|GetNumberSlots)))