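; Collectible item pickup, either mineral or water, that the player character gathers by overlapping it.
; Construction script adds a small mesh with the material matching its type.
; On player overlap, mineral adds Amount to the controller's Mine while water resets Water to zero; both notify the GameMode and award a point.
; The item then destroys itself, calling a Niagara component add after DestroyActor, and also expires on a timer after spawning.
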(event EventBeginPlay
  (Utilities|FlowControl|Sequence
    (:then_0
      (bind _gamemode (CallFunction|CastGameMode))
      (Variables|Reference|SetGameMode _gamemode)
      (bind _character (CallFunction|CastCharacter))
      (Variables|Reference|SetCharacter _character)
      (bind _controller (CallFunction|CastController))
      (Variables|Default|SetController _controller))
    (:then_1
      (Utilities|FlowControl|Delay 2e+01)
      (CallFunction|EffectDestroyActor))))

(event Collision|EventActorBeginOverlap
  (params (OtherActor :type Actor%20Object%20Reference))
  (bind _gamemode (Variables|Reference|GetGameMode))
  (bind _controller (Variables|Default|GetController))
  (if (== OtherActor (Variables|Reference|GetCharacter))
    (switch Utilities|FlowControl|Switch|SwitchonE_Type (Utilities|Struct|BreakS_ItemType (Variables|Default|GetType))
      (:NewEnumerator0
        (bind _output_get (Variables|/Game/Core/Player/PC_Ingame.PC_Ingame_C|SetMine _controller (+ (Variables|/Game/Core/Player/PC_Ingame.PC_Ingame_C|GetMine _controller) (Variables|Default|GetAmount))))
        (Default|IncrementMineralCollectPlayer _gamemode _output_get))
      (:NewEnumerator2
        (bind _output_get_2 (Variables|/Game/Core/Player/PC_Ingame.PC_Ingame_C|SetWater _controller 0.0))
        (Default|IncrementWaterCollectPlayer _gamemode _output_get_2)))
    (Default|AddOnePoints _gamemode)
    (CallFunction|EffectDestroyActor)))

(fn ConstructionScript
  (switch Utilities|FlowControl|Switch|SwitchonE_Type (Utilities|Struct|BreakS_ItemType (Variables|Default|GetType))
    (:NewEnumerator0
      (bind _returnvalue (AddComponent|AddStaticMeshComponent false))
      (Transformation|SetRelativeScale3D _returnvalue "0.200000,0.200000,0.200000")
      (Rendering|Material|SetMaterial _returnvalue 0 "/Game/Core/Item/Mineral/MI_Mineral.MI_Mineral"))
    (:NewEnumerator2
      (bind _returnvalue_2 (AddComponent|AddStaticMeshComponent false))
      (Transformation|SetRelativeScale3D _returnvalue_2 "0.200000,0.200000,0.200000")
      (Rendering|Material|SetMaterial _returnvalue_2 0 "/Game/Core/Item/Water/MI_Water.MI_Water"))))

(fn EffectDestroyActor
  (Actor|DestroyActor)
  (AddComponent|AddNiagaraComponent false)
  (return))